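; Simulation game mode that manages the switch between the in-simulation UI and the edit UI.
; BeginPlay creates both widgets, shows WG_InSim and enables the mouse cursor.
; ChangeUI clears all widgets, flips the Paused flag and shows the matching widget, calling GetValues on WG_EditSim when paused.
; Paused only selects the UI here; the game itself is not paused in this graph.
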(event EventBeginPlay
  (bind _returnvalue (Game|GetPlayerController 0))
  (bind _returnvalue_2 (UserInterface|CreateWidget "/Game/UI/WG_InSim.WG_InSim_C" _returnvalue))
  (bind _output_get (Variables|Default|SetIngame _returnvalue_2))
  (UserInterface|Viewport|AddtoViewport _output_get 0)
  (Variables|/Script/Engine.PlayerController|SetbShowMouseCursor _returnvalue true)
  (bind _returnvalue_3 (UserInterface|CreateWidget "/Game/UI/WG_EditSim.WG_EditSim_C" _returnvalue))
  (Variables|Default|SetEdit _returnvalue_3))

(event Collision|EventActorBeginOverlap
  (params (OtherActor :type Actor%20Object%20Reference)))

(event EventTick
  (params (DeltaSeconds :type Float%20%28single-precision%29)))

(fn ConstructionScript)

(fn ChangeUI
  (bind _edit (Variables|Default|GetEdit))
  (Viewport|RemoveAllWidgets)
  (bind _output_get (Variables|Default|SetPaused (not (Variables|Default|GetPaused))))
  (if _output_get
    (UserInterface|Viewport|AddtoViewport _edit 0)
    (bind _aswg_edit_sim (Utilities|Casting|CastToWG_EditSim _edit))
    (Default|GetValues _aswg_edit_sim)
    (else
      (UserInterface|Viewport|AddtoViewport (Variables|Default|GetIngame) 0))))